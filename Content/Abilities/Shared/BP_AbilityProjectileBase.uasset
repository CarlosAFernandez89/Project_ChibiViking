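; Base projectile actor for abilities that delivers a gameplay effect container to actors it overlaps.
; On overlap it records each new actor in HitActors to avoid repeat hits and excludes its instigator from the effect.
; Valid hits are added as targets to EffectContainerSpec, which is then applied as an external spec, so the projectile itself defines no effect logic.
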(event `self.ReceiveActorBeginOverlap`
  (params (OtherActor :type "Actor Object Reference"))
  (bind _hitactors (`self.HitActors`))
  (if (not (`KismetArrayLibrary.Array_Contains` _hitactors))
    (`KismetArrayLibrary.Array_Add` _hitactors OtherActor)
    (if (!= OtherActor (`self.GetInstigator`))
      (bind _returnvalue (`RPGBlueprintLibrary.AddTargetsToEffectContainerSpec` :`ContainerSpec` (`self.EffectContainerSpec`) :`TargetActors` (`|MakeArray` OtherActor)))
      (`RPGBlueprintLibrary.ApplyExternalEffectContainerSpec` _returnvalue))))

(fn `UserConstructionScript`)