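; Gameplay ability for the player dodge, a roll impulse along the capsule's forward vector.
; On activation it runs the parent logic, then checks CanUseAnyAbility on the player character.
; If allowed and not falling, it stops movement and launches the character additively by RollImpulseForce.
; If blocked, it prints a low-mana or cooldown message based on an attribute threshold; this graph itself neither commits nor ends the ability.
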(event `self.K2_ActivateAbility`
  (bind _controller (`/Game/Blueprints/BP_RPGFunctionLibrary.GetPlayerControllerBP`))
  (bind _mycharacter (`/Game/Blueprints/BP_RPGFunctionLibrary.GetPlayerCharacterBP`))
  (bind _charactermovement (`Character.CharacterMovement` (`/Game/Character/Blueprints/BP_PlayerController.PlayerCharacter` _controller)))
  (`parent.K2_ActivateAbility`)
  (if (`/Game/Character/Blueprints/BP_Character.CanUseAnyAbility` (`/Game/Character/Blueprints/BP_PlayerController.PlayerCharacter` _controller))
    (if (not (`NavMovementComponent.IsFalling` _charactermovement))
      (`MovementComponent.StopMovementImmediately` _charactermovement)
      (`Character.LaunchCharacter` _mycharacter (* (`SceneComponent.GetForwardVector` (`Character.CapsuleComponent` _mycharacter)) (`self.RollImpulseForce`)) false false))
    (elif (< (`.ReturnValue` (`AbilitySystemBlueprintLibrary.GetFloatAttributeFromAbilitySystemComponent` null (struct :`AttributeName` "Mana" :`Attribute` "/Script/GAS_Core.RPGAttributeSet:Mana"))) 25.0)
      (`KismetSystemLibrary.PrintString` "Not enough mana!")
      (else
        (`KismetSystemLibrary.PrintString` "Dodge on Cooldown!")))))