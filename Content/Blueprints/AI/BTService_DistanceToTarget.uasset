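; Behavior tree service that keeps an AI pawn's spatial data current on the Blackboard.
; On search start it caches the controlled pawn, then runs the same update there and on every tick.
; It writes the distance to the TargetToFollow actor into DistToTarget.
; AIForwardVector receives the pawn's location plus its forward vector, a world point one unit ahead rather than a direction.
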(event `self.ReceiveSearchStartAI`
  (params (OwnerController :type "AIController Object Reference") (ControlledPawn :type "Pawn Object Reference"))
  (bind _controlled_pawn (`self.Controlled Pawn`))
  (set `self.Controlled Pawn` ControlledPawn)
  (`BTFunctionLibrary.SetBlackboardValueAsFloat` (`self.DistToTarget`) (`Actor.GetDistanceTo` (`self.Controlled Pawn`) (`BTFunctionLibrary.GetBlackboardValueAsActor` (`self.TargetToFollow`))) :!label _label)
  (`BTFunctionLibrary.SetBlackboardValueAsVector` (`self.AIForwardVector`) (+ (`Actor.K2_GetActorLocation` _controlled_pawn) (`Actor.GetActorForwardVector` _controlled_pawn))))

(event `self.ReceiveTickAI`
  (params (OwnerController :type "AIController Object Reference") (ControlledPawn :type "Pawn Object Reference") (DeltaSeconds :type "Float (single-precision)"))
  (goto _label))