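; Anim notify state that marks a combo window in the player's montage, where the animation can jump to another section.
; On begin and on every tick it calls JumpSectionForCombo on the PlayerCharacter held by the game mode.
; On end it casts the mesh owner to BP_PlayerCharacter and clears EnableComboPeriod.
; Begin and tick therefore always target the game mode's player, whichever mesh plays the animation.
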(fn `Received_NotifyBegin`
  (params (MeshComp :type "SkeletalMeshComponent Object Reference") (Animation :type "AnimSequenceBase Object Reference") (TotalDuration :type "Float (double-precision)"))
  (returns (ReturnValue :type Boolean))
  (bind _playercharacter (`/Game/Character/Blueprints/BP_GameMode.PlayerCharacter` (`/Game/Blueprints/BP_RPGFunctionLibrary.GetGameModeBP` Animation)))
  (`/Engine/EditorBlueprintResources/StandardMacros.IsValid` MeshComp
    (:`Is Valid`
      (`/Engine/EditorBlueprintResources/StandardMacros.IsValid` _playercharacter
        (:`Is Valid`
          (`/Game/Character/Blueprints/BP_PlayerCharacter.JumpSectionForCombo` _playercharacter)
          (return true))))))

(fn `Received_NotifyEnd`
  (params (MeshComp :type "SkeletalMeshComponent Object Reference") (Animation :type "AnimSequenceBase Object Reference"))
  (returns (ReturnValue :type Boolean))
  (bind _asbp_player_character (cast `/Game/Character/Blueprints/BP_PlayerCharacter` (`ActorComponent.GetOwner` MeshComp)))
  (set `/Game/Character/Blueprints/BP_PlayerCharacter.bEnableComboPeriod` false _asbp_player_character)
  (return false))

(fn `Received_NotifyTick`
  (params (MeshComp :type "SkeletalMeshComponent Object Reference") (Animation :type "AnimSequenceBase Object Reference") (FrameDeltaTime :type "Float (double-precision)"))
  (returns (ReturnValue :type Boolean))
  (bind _playercharacter (`/Game/Character/Blueprints/BP_GameMode.PlayerCharacter` (`/Game/Blueprints/BP_RPGFunctionLibrary.GetGameModeBP` MeshComp)))
  (`/Engine/EditorBlueprintResources/StandardMacros.IsValid` Animation
    (:`Is Valid`
      (`/Engine/EditorBlueprintResources/StandardMacros.IsValid` _playercharacter
        (:`Is Valid`
          (`/Game/Character/Blueprints/BP_PlayerCharacter.JumpSectionForCombo` _playercharacter)
          (return true))))))