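; Anim notify state that marks the attack window of a character's current weapon within an animation.
; On begin, it gets the mesh owner's BP_Character weapon, flags it as attacking and calls BeginWeaponAttack with the notify's event tag and delay time and count.
; On end, it calls EndWeaponAttack on the current weapon.
; Both events act only when that weapon is valid.
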(fn `Received_NotifyBegin`
  (params (MeshComp :type "SkeletalMeshComponent Object Reference") (Animation :type "AnimSequenceBase Object Reference") (TotalDuration :type "Float (double-precision)"))
  (returns (ReturnValue :type Boolean))
  (bind _currentweapon (`/Game/Character/Blueprints/BP_Character.CurrentWeapon` (cast `/Game/Character/Blueprints/BP_Character` (`ActorComponent.GetOwner` MeshComp) :!pure true)))
  (`/Engine/EditorBlueprintResources/StandardMacros.IsValid` _currentweapon
    (:`Is Valid`
      (set `/Game/Blueprints/Weapon/WeaponActor.IsAttacking` true _currentweapon)
      (`/Game/Blueprints/Weapon/WeaponActor.BeginWeaponAttack` _currentweapon (`self.Event Tag`) (`self.Attack Delay Time`) (`self.Attack Delay Count`))
      (return true))))

(fn `Received_NotifyEnd`
  (params (MeshComp :type "SkeletalMeshComponent Object Reference") (Animation :type "AnimSequenceBase Object Reference"))
  (returns (ReturnValue :type Boolean))
  (bind _currentweapon (`/Game/Character/Blueprints/BP_Character.CurrentWeapon` (cast `/Game/Character/Blueprints/BP_Character` (`ActorComponent.GetOwner` MeshComp) :!pure true)))
  (`/Engine/EditorBlueprintResources/StandardMacros.IsValid` _currentweapon
    (:`Is Valid`
      (`/Game/Blueprints/Weapon/WeaponActor.EndWeaponAttack` _currentweapon)
      (return false))))