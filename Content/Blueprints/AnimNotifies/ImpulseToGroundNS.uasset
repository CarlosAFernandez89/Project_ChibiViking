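; Anim notify state that launches the owning BP_Character forward along world X and down toward the ground during an animation.
; On begin it applies a large velocity-change impulse through CharacterMovement.
; Each tick while the character is not on the ground, it adds a smaller forward and downward impulse.
; Impulses are fixed world-space vectors that ignore mass and character facing.
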(fn `Received_NotifyBegin`
  (params (MeshComp :type "SkeletalMeshComponent Object Reference") (Animation :type "AnimSequenceBase Object Reference") (TotalDuration :type "Float (double-precision)"))
  (returns (ReturnValue :type Boolean))
  (`CharacterMovementComponent.AddImpulse` (`Character.CharacterMovement` (cast `/Game/Character/Blueprints/BP_Character` (`ActorComponent.GetOwner` MeshComp) :!pure true)) (5000.0 0.0 -500.0) true)
  (return true))

(fn `Received_NotifyTick`
  (params (MeshComp :type "SkeletalMeshComponent Object Reference") (Animation :type "AnimSequenceBase Object Reference") (FrameDeltaTime :type "Float (double-precision)"))
  (returns (ReturnValue :type Boolean))
  (bind _asbp_character (cast `/Game/Character/Blueprints/BP_Character` (`ActorComponent.GetOwner` MeshComp) :!pure true))
  (if (not (`NavMovementComponent.IsMovingOnGround` (`Character.CharacterMovement` _asbp_character)))
    (`CharacterMovementComponent.AddImpulse` (`Character.CharacterMovement` _asbp_character) (200.0 0.0 -250.0) true)
    (return false)))