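; Enemy minion Blueprint: an armed, AI-driven character that reacts visibly to hits.
; On BeginPlay it spawns its weapon onto the hand_r socket and runs the HTN_CompositionExample hierarchical task network on its AI controller.
; On damage it picks a montage by whether the tags include Ability.Melee, plays a random section, spawns a head emitter and snaps its yaw toward the instigator.
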(event `self.ReceiveBeginPlay`
  ;[1 1 1] Begin Play + Attach Weapon
  (`parent.ReceiveBeginPlay`)
  (bind _returnvalue (`|SpawnActorFromClass` (`self.Weapon`) (`self.WeaponTransform`) "AlwaysSpawn" "OverrideRootScale" null null (struct) self))
  (bind _output_get (set `self.CurrentWeapon` _returnvalue))
  (`self.K2_AttachToComponent` _output_get (`self.Mesh`) "hand_r" "KeepRelative" "KeepRelative" "KeepRelative" true)
  (bind _asaicontroller (cast `AIController` (`self.GetController`)))
  (`HTNBlueprintLibrary.RunHTN` _asaicontroller "/Game/Blueprints/AI/HTN_CompositionExample.HTN_CompositionExample"))

(event `self.OnDamaged`
  (params (DamageAmount :type "Float (single-precision)") (HitInfo :type "HitResult Structure (by ref)") (DamageTags :type "GameplayTagContainer Structure (by ref)") (InstigatorCharacter :type "RPGCharacterBase Object Reference") (DamageCauser :type "Actor Object Reference"))
  ;[1 1 1] On Damaged
  (`parent.OnDamaged` DamageAmount HitInfo DamageTags null null)
  (`self.PlayAnimMontage` (select `bool` (`BlueprintGameplayTagLibrary.MatchesAnyTags` (struct :`TagName` "Ability.Melee") DamageTags) :!type "AnimMontage Object Reference") 1.0 (`KismetStringLibrary.Conv_StringToName` (`KismetStringLibrary.Conv_IntToString` (`KismetMathLibrary.RandomIntegerInRange` 0 1))))
  (`GameplayStatics.SpawnEmitterAttached` null (`self.Mesh`) "head")
  (`self.K2_SetActorRotation` (`KismetMathLibrary.MakeRotator` 0.0 0.0 (.yaw (`KismetMathLibrary.FindLookAtRotation` (`self.K2_GetActorLocation`) (`self.K2_GetActorLocation` InstigatorCharacter))))))

(fn `UserConstructionScript`
  (`parent.UserConstructionScript`))