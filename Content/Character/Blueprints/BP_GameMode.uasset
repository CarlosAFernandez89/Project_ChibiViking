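; Game mode that manages game flow: intro cutscene, player start, game over and level restart.
; The intro plays the first Level Sequence actor found in the level as a skippable cutscene, or starts the game directly if none exists.
; Starting spawns the player once via an in-progress flag, and restart delegates to the game instance.
; Game over plays brief slow motion, then pauses and locks input to UI.
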(event `Restart`
  (`/Game/Character/Blueprints/BP_GameInstance.RestartGameLevel` (`/Game/Blueprints/BP_RPGFunctionLibrary.GetGameInstanceBP`) :!label _label))

(event `self.K2_DoRestart`
  (goto _label))

(event `self.K2_OnGameOver`
  (`GameplayStatics.SetGlobalTimeDilation` 0.25)
  (`KismetSystemLibrary.Delay` 0.5)
  (`GameplayStatics.SetGlobalTimeDilation` 1.0)
  (`GameplayStatics.SetGamePaused` true)
  (`WidgetBlueprintLibrary.SetInputMode_UIOnlyEx` (`/Game/Blueprints/BP_RPGFunctionLibrary.GetPlayerControllerBP`) null "LockAlways") ; Block any inputs
)

(event `StartGame`
  (if (not (`self.bGameInProgress`))
    (set `self.bGameInProgress` true)
    (`self.RestartPlayer` (`/Game/Blueprints/BP_RPGFunctionLibrary.GetPlayerControllerBP`))))

(event `PlayDefaultIntroCutscene`
  ;[1 1 1] Look for Level Sequence in this level to play
  (bind _outactors (`GameplayStatics.GetAllActorsOfClass` "/Script/LevelSequence.LevelSequenceActor"))
  (if (`KismetArrayLibrary.Array_IsValidIndex` _outactors)
    (`/Game/Character/Blueprints/BP_PlayerController.PlaySkippableCutscene` (`/Game/Blueprints/BP_RPGFunctionLibrary.GetPlayerControllerBP`) (`LevelSequenceActor.SequencePlayer` (`|GetArrayItem` _outactors)))
    (else
      (`self.StartGame`))))

(event `self.ReceiveBeginPlay`)

(fn `UserConstructionScript`)