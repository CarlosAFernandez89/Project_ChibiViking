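; Camera manager component that adjusts the player's spring-arm camera at drop-offs and fades the character when the camera gets close.
; Each tick, forward and downward line traces from the spring arm check for ground ahead.
; Without a hit, it eases toward a raised edge offset and a look-at rotation to the trace end, enabling pawn control rotation; otherwise it eases back to defaults.
; Camera-to-capsule distance drives the body materials' Opacity parameter.
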(event `self.ReceiveBeginPlay`
  (bind _returnvalue (`self.GetOwner`))
  ;[1 1 1] BeginPlay
  (set `self.Camera` (`Actor.GetComponentByClass` _returnvalue "/Script/Engine.CameraComponent"))
  (set `self.SpringArm` (`Actor.GetComponentByClass` _returnvalue "/Script/Engine.SpringArmComponent"))
  (set `self.EdgeTargetOffset` (+ (`KismetMathLibrary.Conv_RotatorToVector` (`SceneComponent.K2_GetComponentRotation` (`self.SpringArm`))) (0.0 0.0 200.0))))

(event `CheckForDrop_Infront`
  (bind _springarm (`self.SpringArm`))
  (bind _object_types (`self.Object Types`))
  (bind _returnvalue (`SceneComponent.K2_GetComponentLocation` _springarm))
  (bind _returnvalue_2 (+ _returnvalue (* (`KismetMathLibrary.Conv_RotatorToVector` (`SceneComponent.K2_GetComponentRotation` _springarm)) (200.0 200.0 200.0))))
  ;[1 1 1] DropOff
  ;;[1 1 1] Straight line
  (bind (_outhit _returnvalue_3) (`KismetSystemLibrary.LineTraceSingleForObjects` _returnvalue _returnvalue_2 _object_types))
  ;;[1 1 1] LineDown
  (bind (_outhit_2 _returnvalue_4) (`KismetSystemLibrary.LineTraceSingleForObjects` _returnvalue_2 (+ _returnvalue_2 (`self.DropOffDistance`)) _object_types))
  (if _returnvalue_3
    (set `self.DropOffHit?` true)
    (else
      (set `self.DropOffHit?` _returnvalue_4)
      (set `self.DropOffTraceEndLocation` (`KismetMathLibrary.InverseTransformLocation` (`SceneComponent.GetSocketTransform` _springarm "None" "RTS_World") (`.TraceEnd` (`GameplayStatics.BreakHitResult` _outhit_2)))))))

(event `self.ReceiveTick`
  (params (DeltaSeconds :type "Float (single-precision)"))
  (`|ExecutionSequence`
    (:`then_0`
      (`self.CheckForDrop_Infront`))
    (:`then_1`
      (`self.CheckCameraDistanceToPlayer`))
    (:`then_3`
      (`self.HandleCameraMovement`))))

(event `CheckCameraDistanceToPlayer`
  (bind _asbp_player_character (cast `/Game/Character/Blueprints/BP_PlayerCharacter` (`self.GetOwner` (`self.Camera`)) :!pure true))
  ;[1 1 1] FadeMaterials When Close to Character
  (for _array_element (`/Game/Character/Blueprints/BP_PlayerCharacter.BodyMaterials` _asbp_player_character)
    (`MaterialInstanceDynamic.SetScalarParameterValue` _array_element (`self.Opacity`) (`KismetMathLibrary.MapRangeClamped` (`KismetMathLibrary.Vector_Distance` (`SceneComponent.K2_GetComponentLocation` (`self.Camera`)) (`SceneComponent.K2_GetComponentLocation` (`Character.CapsuleComponent` _asbp_player_character))) 90.0 160.0 0.1 1.0))))

(event `HandleCameraMovement`
  (bind _camera (`self.Camera`))
  (bind _camera_2 (`self.Camera`))
  (bind _springarm (`self.SpringArm`))
  (bind _targetoffset (`SpringArmComponent.TargetOffset` _springarm))
  (bind _relativerotation (`SceneComponent.RelativeRotation` _camera_2))
  (`|ExecutionSequence`
    (:`then_0`
      ;[1 0.1621 0] DropOffLogic
      (if (`self.DropOffHit?`)
        (set `SpringArmComponent.TargetOffset` (`KismetMathLibrary.VLerp` _targetoffset (`self.DefaultTargetOffset`) 0.05) _springarm)
        (`SceneComponent.K2_SetRelativeRotation` _camera_2 (`KismetMathLibrary.RLerp` _relativerotation (struct) 0.05 true) false false)
        (set `CameraComponent.bUsePawnControlRotation` false _camera)
        (else
          (set `SpringArmComponent.TargetOffset` (`KismetMathLibrary.VLerp` _targetoffset (`self.EdgeTargetOffset`) 0.05) _springarm)
          (`SceneComponent.K2_SetRelativeRotation` _camera_2 (`KismetMathLibrary.RLerp` _relativerotation (`KismetMathLibrary.FindLookAtRotation` (`SceneComponent.RelativeLocation` _camera_2) (`self.DropOffTraceEndLocation`)) 0.05 true) false false)
          (set `CameraComponent.bUsePawnControlRotation` true _camera))))))